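; AI controller for DefaultAI pawns that runs their behavior tree and feeds it blackboard data.
; On possess, it copies the pawn's Stay and Interact flags to the blackboard and re-syncs them through the pawn's interaction-change delegate.
; AI perception tracks the first-person player, setting an in-sight key and, when sight is lost, recording the player's current location and a recently-seen flag.
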(event OnTargetPerceptionUpdated(AIPerception)
  (params (Actor :type Actor%20Object%20Reference) (Stimulus :type AI%20Stimulus%20Structure))
  (bind _bsuccessfullysensed (Utilities|Struct|BreakAIStimulus Stimulus))
  ;[1 0 0] OnTargetPerceptionUpdated
  (Utilities|Casting|CastToFirstPersonCharacter Actor)
  (AI|Components|Blackboard|SetValueasBool (Variables|Default|GetBlackboard) (Variables|BlackBoardKeyNames|GetPlayerInSightKey) _bsuccessfullysensed)
  (if (not _bsuccessfullysensed)
    (AI|Components|Blackboard|SetValueasVector (Variables|Default|GetBlackboard) (Variables|BlackBoardKeyNames|GetPlayerLastKnownLocationKey) (Transformation|GetActorLocation (Game|GetPlayerCharacter 0)))
    (AI|Components|Blackboard|SetValueasBool (Variables|Default|GetBlackboard) (Variables|BlackBoardKeyNames|GetPlayerRecentlyInSightKey) true)))

(event Custom|SetupInteraction
  (AI|Components|Blackboard|SetValueasBool (Variables|Default|GetBlackboard) (Variables|BlackBoardKeyNames|GetAIStayKey) (Variables|/Game/Blueprints/DefaultAI.DefaultAI_C|GetbStay (Variables|Default|GetDefault%20AI)))
  (AI|Components|Blackboard|SetValueasBool (Variables|Default|GetBlackboard) (Variables|BlackBoardKeyNames|GetInteractKey) (Variables|/Game/Blueprints/DefaultAI.DefaultAI_C|GetbInteract (Variables|Default|GetDefault%20AI))))

(event EventPossess
  (params (PossessedPawn :type Pawn%20Object%20Reference))
  ;[0.01925 0 1] SetDefaultValues
  (bind _asdefault_ai (Utilities|Casting|CastToDefaultAI PossessedPawn))
  (Variables|Default|SetDefault%20AI _asdefault_ai)
  (AI|RunBehaviorTree "/Game/Blueprints/AI/DefaultAITree.DefaultAITree")
  (CallFunction|SetupInteraction)
  (EventDispatchers|AssignInteractionChange (Variables|Default|GetDefault%20AI) (delegate Custom|SetupInteraction)))

(fn ConstructionScript)