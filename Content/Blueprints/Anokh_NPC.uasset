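; Anokh NPC actor that starts its dialog and turns the player's view toward itself when approached.
; A sphere overlap by the first-person character calls AnokhDialog, passing the NPC's first InteractionInterface component.
; After a short delay, a timeline lerps control rotation from the current camera rotation to face the NPC.
; When the timeline finishes, it sets HasInteracted to block repeats and clears BeforeStay.
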(event OnComponentBeginOverlap(Sphere)
  (params (OverlappedComponent :type Primitive%20Component%20Object%20Reference) (OtherActor :type Actor%20Object%20Reference) (OtherComp :type Primitive%20Component%20Object%20Reference) (OtherBodyIndex :type Integer) (bFromSweep :type Boolean) (SweepResult :type Hit%20Result%20Structure%20%28by%20ref%29))
  (if (not (Variables|Default|GetbHasInteracted))
    (bind _asfirst_person_character (Utilities|Casting|CastToFirstPersonCharacter OtherActor))
    (Default|AnokhDialog _asfirst_person_character (Utilities|Array|Get(acopy) (Class|Actor|GetComponentsbyInterface "/Game/FirstPersonBP/Blueprints/Dialog/InteractionInterface.InteractionInterface_C")))
    (Variables|Default|SetLerpStart (Transformation|GetWorldRotation (Variables|/Game/FirstPersonBP/Blueprints/FirstPersonCharacter.FirstPersonCharacter_C|GetFirstPersonCamera _asfirst_person_character)))
    (Variables|Default|SetLerpEnd (Math|Rotator|FindLookatRotation (Transformation|GetWorldLocation (Variables|/Game/FirstPersonBP/Blueprints/FirstPersonCharacter.FirstPersonCharacter_C|GetFirstPersonCamera _asfirst_person_character)) (Transformation|GetActorLocation)))
    (Utilities|FlowControl|Delay 0.2)
    (bind _alpha (Timeline|PlayerLookAt Play)
      (:Update
        (Pawn|SetControlRotation (Game|GetPlayerController 0) (Math|Rotator|Lerp(Rotator) (Variables|Default|GetLerpStart) (Variables|Default|GetLerpEnd) _alpha)))
      (:Finished
        (Variables|Default|SetbHasInteracted true)
        (Variables|Default|SetbBeforeStay false)))))

(event EventBeginPlay
  (|CallParentFunction) ; This node is disabled and will not be called.\nDrag off pins to build functionality.
)

(event Collision|EventActorBeginOverlap
  (params (OtherActor :type Actor%20Object%20Reference)))

(event EventTick
  (params (DeltaSeconds :type Float%20%28single-precision%29)))

(fn ConstructionScript
  (|CallParentFunction))