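; DefaultAI is an AI character Blueprint that pauses for dialog interactions and switches between walk and run speeds.
; On BeginPlay it binds to DialogComponent interaction events, setting Stay and Interact, broadcasting the change, and restoring the prior Stay state on exit.
; Walk and Run events set the movement max speed.
; The construction script makes rotation follow the controller's desired rotation smoothly rather than movement direction.
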(event Custom|Interaction
  (Variables|CharacterStats|SetbBeforeStay (Variables|CharacterStats|GetbStay))
  (Variables|CharacterStats|SetbStay true)
  (Variables|CharacterStats|SetbInteract true)
  (Default|CallInteractionChange))

(event Custom|ExitInteraction
  (Variables|CharacterStats|SetbStay (Variables|CharacterStats|GetbBeforeStay))
  (Variables|CharacterStats|SetbInteract false)
  (Default|CallInteractionChange))

(event Custom|Walk
  (Variables|/Script/Engine.CharacterMovementComponent|SetMaxWalkSpeed (Variables|Character|GetCharacterMovement) (Variables|CharacterStats|GetWalkSpeed)))

(event Custom|Run
  (Variables|/Script/Engine.CharacterMovementComponent|SetMaxWalkSpeed (Variables|Character|GetCharacterMovement) (Variables|CharacterStats|GetRunSpeed)))

(event EventBeginPlay
  (EventDispatchers|BindEventtoOnInteractionCall (Variables|Default|GetDialogComponent) (delegate Custom|Interaction))
  (EventDispatchers|BindEventtoOnInteractionExit (Variables|Default|GetDialogComponent) (delegate Custom|ExitInteraction)))

(fn ConstructionScript
  (Variables|Default|SetbUseControllerRotationYaw false)
  (Variables|/Script/Engine.CharacterMovementComponent|SetbOrientRotationToMovement (Variables|Character|GetCharacterMovement) false)
  (Variables|/Script/Engine.CharacterMovementComponent|SetbUseControllerDesiredRotation (Variables|Character|GetCharacterMovement) true)
  (Variables|/Script/Engine.CharacterMovementComponent|SetRotationRate (Variables|Character|GetCharacterMovement) "0,540.000000, 0"))