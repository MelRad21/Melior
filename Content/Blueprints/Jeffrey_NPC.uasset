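; Jeffrey NPC that opens a forced dialog with the player on BeginPlay if it has not yet been interacted with.
; It passes its interaction component to the first-person character, then after a short delay a timeline lerps the player's control rotation to face Jeffrey.
; When the turn finishes it marks itself interacted and binds a one-shot dialog-exit handler that clears Yi's stay flags and triggers Yi's interaction change.
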(event Custom|RecallYi
  (bind _yi (Variables|Default|GetYi))
  (bind _output (Utilities|ResolveSoftReference _yi))
  (Variables|/Game/Blueprints/DefaultAI.DefaultAI_C|SetbStay _output false)
  (Variables|/Game/Blueprints/DefaultAI.DefaultAI_C|SetbBeforeStay _output false)
  (Default|CallInteractionChange _output)
  (EventDispatchers|UnbindEventfromOnInteractionExit (Variables|Default|GetDialogComponent) (delegate Custom|RecallYi)))

(event EventBeginPlay
  (|CallParentFunction)
  (if (not (Variables|Default|GetbHasInteracted))
    (bind _asfirst_person_character (Utilities|Casting|CastToFirstPersonCharacter (Game|GetPlayerCharacter 0)))
    (Default|AnokhDialog _asfirst_person_character (Utilities|Array|Get(acopy) (Class|Actor|GetComponentsbyInterface "/Game/FirstPersonBP/Blueprints/Dialog/InteractionInterface.InteractionInterface_C")))
    (Variables|Default|SetLerpStart (Transformation|GetWorldRotation (Variables|/Game/FirstPersonBP/Blueprints/FirstPersonCharacter.FirstPersonCharacter_C|GetFirstPersonCamera _asfirst_person_character)))
    (Variables|Default|SetLerpEnd (Math|Rotator|FindLookatRotation (Transformation|GetWorldLocation (Variables|/Game/FirstPersonBP/Blueprints/FirstPersonCharacter.FirstPersonCharacter_C|GetFirstPersonCamera _asfirst_person_character)) (Transformation|GetActorLocation)))
    (Utilities|FlowControl|Delay 0.2)
    (bind _alpha (Timeline|Timeline_0 Play)
      (:Update
        (Pawn|SetControlRotation (Game|GetPlayerController 0) (Math|Rotator|Lerp(Rotator) (Variables|Default|GetLerpStart) (Variables|Default|GetLerpEnd) _alpha)))
      (:Finished
        (Variables|Default|SetbHasInteracted true)
        (Variables|Default|SetbBeforeStay false)
        (EventDispatchers|BindEventtoOnInteractionExit (Variables|Default|GetDialogComponent) (delegate Custom|RecallYi))))))

(event Collision|EventActorBeginOverlap
  (params (OtherActor :type Actor%20Object%20Reference)))

(event EventTick
  (params (DeltaSeconds :type Float%20%28single-precision%29)))

(fn ConstructionScript
  (|CallParentFunction))